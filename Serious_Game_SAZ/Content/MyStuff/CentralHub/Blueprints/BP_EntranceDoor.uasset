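; BP_EntranceDoor is a central hub door actor that sends the game into a level when its ExitZone is overlapped.
; On BeginPlay it checks the GI_MinigameProgress game instance for its LevelName among CompletedGames.
; Completed entries hide the door and disable the zone's collision, so that level can no longer be entered through it.
; The overlap opens the referenced Level without filtering which actor triggered it.
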(event OnComponentBeginOverlap(ExitZone)
  (params (OverlappedComponent :type Primitive%20Component%20Object%20Reference) (OtherActor :type Actor%20Object%20Reference) (OtherComp :type Primitive%20Component%20Object%20Reference) (OtherBodyIndex :type Integer) (bFromSweep :type Boolean) (SweepResult :type Hit%20Result%20Structure%20%28by%20ref%29))
  (Game|OpenLevel(byObjectReference) (Variables|Default|GetLevel)))

(event EventBeginPlay
  (bind _asgi_minigame_progress (Utilities|Casting|CastToGI_MinigameProgress (Game|GetGameInstance)))
  (if (Utilities|Array|ContainsItem (Variables|/Game/MyStuff/CentralHub/Blueprints/GI_MinigameProgress.GI_MinigameProgress_C|GetCompletedGames _asgi_minigame_progress) (Variables|Default|GetLevelName))
    (Rendering|SetActorHiddenInGame true)
    (Collision|SetCollisionEnabled (Variables|Default|GetExitZone) "NoCollision")))

(event Collision|EventActorBeginOverlap
  (params (OtherActor :type Actor%20Object%20Reference)))

(event EventTick
  (params (DeltaSeconds :type Float%20%28single-precision%29)))

(fn ConstructionScript)