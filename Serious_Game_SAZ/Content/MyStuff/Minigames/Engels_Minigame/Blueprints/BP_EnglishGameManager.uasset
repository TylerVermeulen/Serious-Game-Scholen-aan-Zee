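; Manager actor for the English vocabulary minigame, where players answer timed questions by selecting orbiting words.
; It shows a tutorial, loads shuffled questions from a difficulty-specific DataTable, then spawns answers as BP_WordTarget actors circling the player in alternating directions and heights.
; Correct picks score; a timeout or third miss advances the question.
; EndGame records completion in GI_MinigameProgress, awards a point at a hardcoded threshold and shows the end screen.
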(event EventBeginPlay
  (Utilities|FlowControl|Delay 0.1)
  (CallFunction|ShowTutorial))

(fn ConstructionScript)

(fn WordSelected
  (params (SelectedWord :type Name) (SelectedActor :type BP%20Word%20Target%20Object%20Reference))
  (if (== SelectedWord (.correctanswer (Variables|Default|GetCurrentQuestion)))
    (Variables|Default|SetScore (+ (Variables|Default|GetScore) 1))
    (Default|ConsumeCorrectly SelectedActor)
    (Audio|PlaySound2D "/Game/MyStuff/Minigames/Geschiedenis_Minigame/Audio/SW_Correct.SW_Correct" 1.0 1.0 0.0 0 0)
    (Utilities|Time|ClearandInvalidateTimerbyHandle (Variables|Default|GetQuestionTimerHandle) :!label _label)
    (CallFunction|NextQuestion)
    (else
      (Variables|Default|SetAttempts (+ (Variables|Default|GetAttempts) 1))
      (if (>= (Variables|Default|GetAttempts) 3)
        (Audio|PlaySound2D "/Game/MyStuff/Minigames/Geschiedenis_Minigame/Audio/SW_Incorrect.SW_Incorrect" 1.0 1.0 0.0 0 0)
        (goto _label)
        (else
          (Default|HideforQuestion SelectedActor))))))

(fn StartMinigame
  (Variables|Default|SetbGameActive true)
  (CallFunction|LoadQuestions)
  (CallFunction|SpawnWords)
  (bind _returnvalue (UserInterface|CreateWidget "/Game/MyStuff/Minigames/Engels_Minigame/UI/WBP_EnglishQuestion.WBP_EnglishQuestion_C"))
  (bind _output_get (Variables|Default|SetQuestionWidget _returnvalue))
  (UserInterface|Viewport|AddtoViewport _output_get 0)
  (CallFunction|StartQuestion))

(fn SpawnWords
  (bind _spawnradius (Variables|Default|GetSpawnRadius))
  (Variables|Default|SetPlayerLocation (Transformation|GetActorLocation (Game|GetPlayerCharacter 0)))
  (for (_array_element _array_index) (Variables|Default|GetWordBank)
    (bind _output_get (Variables|Default|SetAngle (* (/ 360 (Utilities|Array|Length (Variables|Default|GetWordBank))) _array_index)))
    (bind _returnvalue (Game|SpawnActorfromClass "/Game/MyStuff/Minigames/Engels_Minigame/Blueprints/BP_WordTarget.BP_WordTarget_C" (Math|Transform|MakeTransform (+ (Math|Vector|MakeVector (* (Math|Trig|Cos(Radians) (Math|Trig|DegreesToRadians (Math|Conversions|ToFloat(Integer) _output_get))) _spawnradius) (* (Math|Trig|Sin(Radians) (Math|Trig|DegreesToRadians (Math|Conversions|ToFloat(Integer) _output_get))) _spawnradius) (Math|Random|RandomFloatinRange 5e+01 2.5e+02)) (Variables|Default|GetPlayerLocation)) "0, 0, 0" "1.000000,1.000000,1.000000") "Undefined" "MultiplyWithRoot" 0 0))
    (Default|InitializeWord _returnvalue _array_element self)
    (if (== (Math|Integer|%(Integer) _array_index 2) 0)
      (Variables|/Game/MyStuff/Minigames/Engels_Minigame/Blueprints/BP_WordTarget.BP_WordTarget_C|SetOrbitHeight _returnvalue (Math|Random|RandomFloatinRange 275.0 3.5e+02))
      (Variables|/Game/MyStuff/Minigames/Engels_Minigame/Blueprints/BP_WordTarget.BP_WordTarget_C|SetOrbitSpeed _returnvalue 35.0)
      (else
        (Variables|/Game/MyStuff/Minigames/Engels_Minigame/Blueprints/BP_WordTarget.BP_WordTarget_C|SetOrbitHeight _returnvalue (Math|Random|RandomFloatinRange 5e+01 125.0))
        (Variables|/Game/MyStuff/Minigames/Engels_Minigame/Blueprints/BP_WordTarget.BP_WordTarget_C|SetOrbitSpeed _returnvalue -35.0)))
    (Variables|/Game/MyStuff/Minigames/Engels_Minigame/Blueprints/BP_WordTarget.BP_WordTarget_C|SetOrbitAngle _returnvalue (Math|Conversions|ToFloat(Integer) (* (/ 360 (Utilities|Array|Length (Variables|Default|GetWordBank))) _array_index)))
    (Utilities|Array|Add (Variables|Default|GetWordActors) _returnvalue)))

(fn StartQuestion
  (bind _questionwidget (Variables|Default|GetQuestionWidget))
  (bind _output_get (Variables|Default|SetCurrentQuestion (Utilities|Array|Get(acopy) (Variables|Default|GetQuestions) (Variables|Default|GetCurrentQuestionIndex))))
  (Default|UpdateQuestion _questionwidget (.questiontext _output_get))
  (Default|UpdateScore _questionwidget (Variables|Default|GetScore))
  (Variables|Default|SetTimeRemaining (.timelimit (Variables|Default|GetCurrentQuestion)))
  (for _array_element (Variables|Default|GetWordActors)
    (Utilities|IsValid _array_element
      (:Is%20Valid
        (if (not (Variables|/Game/MyStuff/Minigames/Engels_Minigame/Blueprints/BP_WordTarget.BP_WordTarget_C|GetbPermanentlyRemoved _array_element))
          (Default|ShowforQuestion _array_element)))))
  (bind _returnvalue (Utilities|Time|SetTimerbyFunctionName 0 "TickQuestionTimer" 1.0 true))
  (Variables|Default|SetQuestionTimerHandle _returnvalue))

(fn TickQuestionTimer
  (bind _output_get (Variables|Default|SetTimeRemaining (- (Variables|Default|GetTimeRemaining) 1.0)))
  (Default|UpdateTimer (Variables|Default|GetQuestionWidget) _output_get)
  (if (<= _output_get 0.0)
    (Utilities|Time|ClearandInvalidateTimerbyHandle (Variables|Default|GetQuestionTimerHandle))
    (CallFunction|NextQuestion)))

(fn NextQuestion
  (Variables|Default|SetCurrentQuestionIndex (+ (Variables|Default|GetCurrentQuestionIndex) 1))
  (Variables|Default|SetAttempts 0)
  (if (>= (Variables|Default|GetCurrentQuestionIndex) (Utilities|Array|Length (Variables|Default|GetQuestions)))
    (CallFunction|EndGame)
    (else
      (CallFunction|StartQuestion))))

(fn EndGame
  (Variables|Default|SetbGameActive false)
  (Utilities|Time|ClearandInvalidateTimerbyHandle (Variables|Default|GetQuestionTimerHandle))
  (bind _asgi_minigame_progress (Utilities|Casting|CastToGI_MinigameProgress (Game|GetGameInstance)))
  (Variables|/Game/MyStuff/CentralHub/Blueprints/GI_MinigameProgress.GI_MinigameProgress_C|SetbEnglishDone _asgi_minigame_progress true)
  (Utilities|Array|AddUnique (Variables|/Game/MyStuff/CentralHub/Blueprints/GI_MinigameProgress.GI_MinigameProgress_C|GetCompletedGames _asgi_minigame_progress) "EngelsGame")
  (if (>= (Variables|Default|GetScore) 15)
    (Variables|/Game/MyStuff/CentralHub/Blueprints/GI_MinigameProgress.GI_MinigameProgress_C|SetTotalPoints _asgi_minigame_progress (+ (Variables|/Game/MyStuff/CentralHub/Blueprints/GI_MinigameProgress.GI_MinigameProgress_C|GetTotalPoints _asgi_minigame_progress) 1)))
  (bind _returnvalue (UserInterface|CreateWidget "/Game/MyStuff/Minigames/Engels_Minigame/UI/WBP_GameEnd.WBP_GameEnd_C" (Game|GetPlayerController 0)))
  (Variables|Default|SetGameEndWidget _returnvalue)
  (if (>= (Variables|Default|GetScore) (Variables|Default|GetRequiredScore))
    (Widget|SetVisibility (Variables|/Game/MyStuff/Minigames/Engels_Minigame/UI/WBP_GameEnd.WBP_GameEnd_C|GetTextBlock_Opperpoint (Variables|Default|GetGameEndWidget)) "Visible")
    (else
      (Widget|SetVisibility (Variables|/Game/MyStuff/Minigames/Engels_Minigame/UI/WBP_GameEnd.WBP_GameEnd_C|GetTextBlock_Opperpoint (Variables|Default|GetGameEndWidget)) "Hidden")))
  (UserInterface|Viewport|AddtoViewport (Variables|Default|GetGameEndWidget) 0)
  (Input|SetInputModeUIOnly (Game|GetPlayerController 0) (Variables|Default|GetGameEndWidget) "DoNotLock" false)
  (Variables|/Script/Engine.PlayerController|SetbShowMouseCursor (Game|GetPlayerController 0) true))

(fn LoadQuestions
  (switch Utilities|FlowControl|Switch|SwitchonE_EnglishDifficulty (Variables|Default|GetSelectedDifficulty)
    (:NewEnumerator0
      (Variables|Default|SetQuestionTable "/Game/MyStuff/Minigames/Engels_Minigame/Data/DT_EnglishQuestionsEasy.DT_EnglishQuestionsEasy"))
    (:NewEnumerator1
      (Variables|Default|SetQuestionTable "/Game/MyStuff/Minigames/Engels_Minigame/Data/DT_EnglishQuestionMedium.DT_EnglishQuestionMedium"))
    (:NewEnumerator2
      (Variables|Default|SetQuestionTable "/Game/MyStuff/Minigames/Engels_Minigame/Data/DT_EnglishQuestionHard.DT_EnglishQuestionHard")))
  (bind _outrownames (DataTable|GetDataTableRowNames (Variables|Default|GetQuestionTable)))
  (for _array_element _outrownames
    (bind _returnvalue (Utilities|GetDataTableRow (Variables|Default|GetQuestionTable) _array_element)
      (:then
        (Utilities|Array|Add (Variables|Default|GetQuestions) _returnvalue)
        (Utilities|Array|Shuffle (Variables|Default|GetQuestions)))))
  (for _array_element_2 (Variables|Default|GetQuestions)
    (Utilities|Array|Add (Variables|Default|GetWordBank) (.correctanswer _array_element_2))
    (Utilities|Array|Shuffle (Variables|Default|GetWordBank))))

(fn ShowDifficultyMenu
  (bind _returnvalue (Game|GetPlayerController 0))
  (bind _returnvalue_2 (UserInterface|CreateWidget "/Game/MyStuff/Minigames/Engels_Minigame/UI/WBP_DifficultySelect.WBP_DifficultySelect_C" 0 self))
  (UserInterface|Viewport|AddtoViewport _returnvalue_2 0)
  (Input|SetInputModeUIOnly _returnvalue _returnvalue_2 "DoNotLock" false)
  (Variables|/Script/Engine.PlayerController|SetbShowMouseCursor _returnvalue true))

(fn ShowTutorial
  (bind _returnvalue (Game|GetPlayerController 0))
  (bind _returnvalue_2 (UserInterface|CreateWidget "/Game/MyStuff/Minigames/Engels_Minigame/UI/WBP_Tutorial.WBP_Tutorial_C" 0 self))
  (UserInterface|Viewport|AddtoViewport _returnvalue_2 0)
  (Input|SetInputModeUIOnly _returnvalue _returnvalue_2 "DoNotLock" false)
  (Variables|/Script/Engine.PlayerController|SetbShowMouseCursor _returnvalue true))