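; BP_WordTarget is a hittable word target for the Engels minigame that orbits a center point while turning toward the player camera.
; InitializeWord stores the word and manager reference, then shows the text on its WBP_WordTarget widget.
; HitWord reports the word and actor to that manager.
; Visibility and box collision toggle together to hide or show it between questions, while ConsumeCorrectly permanently removes and destroys it.
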(event EventTick
  (params (DeltaSeconds :type Float%20%28single-precision%29))
  (bind _orbitradius (Variables|Default|GetOrbitRadius))
  (Transformation|SetWorldRotation (Variables|Default|GetDefaultSceneRoot) (Math|Rotator|FindLookatRotation (Transformation|GetActorLocation) (Camera|GetCameraLocation (Variables|/Script/Engine.PlayerController|GetPlayerCameraManager (Game|GetPlayerController 0)))) false false)
  (bind _output_get (Variables|Default|SetOrbitAngle (+ (Variables|Default|GetOrbitAngle) (* DeltaSeconds (Variables|Default|GetOrbitSpeed)))))
  (Transformation|SetActorLocation (+ (Variables|Default|GetOrbitCenter) (Math|Vector|MakeVector (* (Math|Trig|Cos(Radians) (Math|Trig|DegreesToRadians _output_get)) _orbitradius) (* _orbitradius (Math|Trig|Sin(Radians) (Math|Trig|DegreesToRadians _output_get))) (Variables|Default|GetOrbitHeight))) false false))

(fn ConstructionScript)

(fn InitializeWord
  (params (NewWordText :type Name) (ManagerRef :type BP%20English%20Game%20Manager%20Object%20Reference))
  (Variables|Default|SetWordText NewWordText)
  (Variables|Default|SetOwningManager ManagerRef)
  (bind _aswbp_word_target (Utilities|Casting|CastToWBP_WordTarget (UserInterface|GetUserWidgetObject (Variables|Default|GetWidget))))
  (Default|SetWordText _aswbp_word_target (Variables|Default|GetWordText))
  (Rendering|SetActorHiddenInGame false)
  (Collision|SetCollisionEnabled (Variables|Default|GetBox) "QueryOnly")
  (Variables|Default|SetbTemporarilyHidden false)
  (Variables|Default|SetbPermanentlyRemoved false))

(fn HideforQuestion
  (Rendering|SetActorHiddenInGame true)
  (Collision|SetCollisionEnabled (Variables|Default|GetBox) "NoCollision")
  (Variables|Default|SetbTemporarilyHidden true))

(fn ShowforQuestion
  (if (== (Variables|Default|GetbPermanentlyRemoved) false)
    (Rendering|SetActorHiddenInGame false)
    (Collision|SetCollisionEnabled (Variables|Default|GetBox) "QueryOnly")
    (Variables|Default|SetbTemporarilyHidden false)))

(fn ConsumeCorrectly
  (Variables|Default|SetbPermanentlyRemoved true)
  (Rendering|SetActorHiddenInGame true)
  (Collision|SetCollisionEnabled (Variables|Default|GetBox) "NoCollision")
  (Actor|DestroyActor))

(fn HitWord
  (Utilities|IsValid (Variables|Default|GetOwningManager)
    (:Is%20Valid
      (Default|WordSelected (Variables|Default|GetOwningManager) (Variables|Default|GetWordText) self))))