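; Crafting desk for the biology minigame, where the player places two held items and interacts again to combine them.
; Interact branches on a desk state derived from slot flags and the held item: fill slot A, fill slot B, craft, or collect the result.
; CombineItems matches DT_Recipes rows in either input order, clearing both slots even without a match.
; Dynamic materials on three item visuals show the icons.
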(event EventBeginPlay
  (bind _outrownames (DataTable|GetDataTableRowNames "/Game/MyStuff/Minigames/Biologie_Minigame/Data/DT_Recipes.DT_Recipes"))
  (for _array_element _outrownames
    (bind _returnvalue (Utilities|GetDataTableRow "/Game/MyStuff/Minigames/Biologie_Minigame/Data/DT_Recipes.DT_Recipes" _array_element)
      (:then
        (Utilities|Array|Add (Variables|Default|GetRecipes) _returnvalue)))))

(event Collision|EventActorBeginOverlap
  (params (OtherActor :type Actor%20Object%20Reference)))

(event EventTick
  (params (DeltaSeconds :type Float%20%28single-precision%29)))

(event EventInteract
  (params (Interactor :type BP%20Biologie%20First%20Person%20Character%20Object%20Reference))
  ;[0.15 0.15 0.15 0.5] Checks state on interact and does corresponding thing
  (Variables|Default|SetPlayer Interactor)
  (bind _deskstate (CallFunction|GetDeskState))
  (switch Utilities|FlowControl|Switch|SwitchonE_DeskState _deskstate
    (:NewEnumerator0
      ;[0.15 0.15 0.15 0.5] Places item on corresponding slot
      (Variables|Default|SetSlotAData (Variables|/Game/MyStuff/Minigames/Biologie_Minigame/Blueprints/BP_BiologieFirstPersonCharacter.BP_BiologieFirstPersonCharacter_C|GetHeldItemData (Variables|Default|GetPlayer)))
      (Variables|Default|SetbSlotAOccupied true)
      (Default|ClearHeldItem (Variables|Default|GetPlayer))
      (Rendering|Material|SetTextureParameterValue (Variables|Default|GetPlaneMaterialA) "ItemTexture" (.icon (Variables|Default|GetSlotAData))))
    (:NewEnumerator1
      (Variables|Default|SetSlotBData (Variables|/Game/MyStuff/Minigames/Biologie_Minigame/Blueprints/BP_BiologieFirstPersonCharacter.BP_BiologieFirstPersonCharacter_C|GetHeldItemData (Variables|Default|GetPlayer)))
      (Variables|Default|SetbSlotBOccupied true)
      (Default|ClearHeldItem (Variables|Default|GetPlayer))
      (Rendering|Material|SetTextureParameterValue (Variables|Default|GetPlaneMaterialB) "ItemTexture" (.icon (Variables|Default|GetSlotBData))))
    (:NewEnumerator2
      ;[0.15 0.15 0.15 0.5] Crafts item based on items slotted in desk
      (bind (_resultitem _bfoundrecipe) (CallFunction|CombineItems (Variables|Default|GetSlotAData) (Variables|Default|GetSlotBData)))
      (if _bfoundrecipe
        (bind _output_get (Variables|Default|SetResultData _resultitem))
        (Rendering|Material|SetTextureParameterValue (Variables|Default|GetPlaneMaterialResult) "ItemTexture" (.icon _output_get))
        (Variables|Default|SetbHasResultReady true)))
    (:NewEnumerator3
      ;[0.15 0.15 0.15 0.5] Players picks up crafted item
      (if (not (Variables|/Game/MyStuff/Minigames/Biologie_Minigame/Blueprints/BP_BiologieFirstPersonCharacter.BP_BiologieFirstPersonCharacter_C|GetbHasItem (Variables|Default|GetPlayer)))
        (Default|PickupItemData (Variables|Default|GetPlayer) (Variables|Default|GetResultData))
        (Variables|Default|SetResultData "")
        (Variables|Default|SetbHasResultReady false)
        (Rendering|Material|SetTextureParameterValue (Variables|Default|GetPlaneMaterialResult) "ItemTexture" "/Game/MyStuff/Minigames/Biologie_Minigame/UI/Sprites/InventoryUI.InventoryUI")
        (else
          (Development|PrintString "hands full"))))))

(fn ConstructionScript
  (bind _returnvalue (Rendering|Material|CreateDynamicMaterialInstance (Variables|Default|GetItemVisualA) 0 "/Game/MyStuff/Minigames/Biologie_Minigame/Materials/M_ItemDisplay.M_ItemDisplay" "None" :!class /Script/Engine.PrimitiveComponent))
  (Variables|Default|SetPlaneMaterialA _returnvalue)
  (bind _returnvalue_2 (Rendering|Material|CreateDynamicMaterialInstance (Variables|Default|GetItemVisualB) 0 "/Game/MyStuff/Minigames/Biologie_Minigame/Materials/M_ItemDisplay.M_ItemDisplay" "None" :!class /Script/Engine.PrimitiveComponent))
  (Variables|Default|SetPlaneMaterialB _returnvalue_2)
  (bind _returnvalue_3 (Rendering|Material|CreateDynamicMaterialInstance (Variables|Default|GetItemVisualResult) 0 "/Game/MyStuff/Minigames/Biologie_Minigame/Materials/M_ItemDisplay.M_ItemDisplay" "None" :!class /Script/Engine.PrimitiveComponent))
  (Variables|Default|SetPlaneMaterialResult _returnvalue_3))

(fn GetDeskState
  (bind _player (Variables|Default|GetPlayer))
  (bind _helditemdata (Variables|/Game/MyStuff/Minigames/Biologie_Minigame/Blueprints/BP_BiologieFirstPersonCharacter.BP_BiologieFirstPersonCharacter_C|GetHeldItemData _player))
  (bind _returnvalue (!= (.itemid _helditemdata) ""))
  ;[0.15 0.15 0.15 0.5] Sets deskstate based on if items are taking a spot or not
  (if (Variables|Default|GetbHasResultReady)
    (return "NewEnumerator3")
    (elif (and (Variables|Default|GetbSlotAOccupied) (Variables|Default|GetbSlotBOccupied))
      (return "NewEnumerator2")
      (elif (or (Variables|Default|GetbSlotAOccupied) (Variables|Default|GetbSlotBOccupied))
        (if _returnvalue
          (return "NewEnumerator1"))
        (elif _returnvalue
          (return "NewEnumerator0"))))))

(fn CombineItems
  (params (ItemA :type ST%20Item%20Data%20Structure) (ItemB :type ST%20Item%20Data%20Structure))
  (LocalVariables|SetLocal_FoundRecipe false)
  (bind _array_element (Utilities|Array|ForEachLoopwithBreak (Variables|Default|GetRecipes))
    (:LoopBody
      (if (not (LocalVariables|GetLocal_FoundRecipe))
        ;[0.15 0.15 0.15 0.5] Clears items on desk so player can place new items
        (if (or (and (== (.itemid ItemA) (.itemid (.inputa _array_element))) (== (.itemid ItemB) (.itemid (.inputb _array_element)))) (and (== (.itemid ItemA) (.itemid (.inputb _array_element))) (== (.itemid ItemB) (.itemid (.inputa _array_element)))))
          (Variables|Default|SetSlotAData "")
          (Variables|Default|SetSlotBData "")
          (Variables|Default|SetbSlotAOccupied false)
          (Variables|Default|SetbSlotBOccupied false)
          (Rendering|Material|SetTextureParameterValue (Variables|Default|GetPlaneMaterialA) "ItemTexture" "/Game/MyStuff/Minigames/Biologie_Minigame/UI/Sprites/InventoryUI.InventoryUI")
          (Rendering|Material|SetTextureParameterValue (Variables|Default|GetPlaneMaterialB) "ItemTexture" "/Game/MyStuff/Minigames/Biologie_Minigame/UI/Sprites/InventoryUI.InventoryUI")
          ;[0.15 0.15 0.15 0.5] Sets the result item to the crafted item
          (LocalVariables|SetLocal_ResultItem (.result _array_element))
          (LocalVariables|SetLocal_FoundRecipe true)
          (else
            (Variables|Default|SetSlotAData "")
            (Variables|Default|SetSlotBData "")
            (Variables|Default|SetbSlotAOccupied false)
            (Variables|Default|SetbSlotBOccupied false)
            (Rendering|Material|SetTextureParameterValue (Variables|Default|GetPlaneMaterialA) "ItemTexture" "/Game/MyStuff/Minigames/Biologie_Minigame/UI/Sprites/InventoryUI.InventoryUI")
            (Rendering|Material|SetTextureParameterValue (Variables|Default|GetPlaneMaterialB) "ItemTexture" "/Game/MyStuff/Minigames/Biologie_Minigame/UI/Sprites/InventoryUI.InventoryUI")))
        (else
          (Utilities|Array|ForEachLoopwithBreak 0) ; enters at Break
        )))
    (:Completed
      (return (LocalVariables|GetLocal_ResultItem) (LocalVariables|GetLocal_FoundRecipe)))))