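; BP_RecipeBook is an interactable recipe book actor in the Biologie minigame that opens an on-screen recipe UI.
; Interact responds only to the Biologie first-person character, creating WBP_RecipeBook when no widget is stored, then switching input to UI-only with a visible cursor.
; When a widget is already stored, interacting only clears that reference, without removing the widget or restoring input.
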(event EventBeginPlay)

(event Collision|EventActorBeginOverlap
  (params (OtherActor :type Actor%20Object%20Reference)))

(event EventTick
  (params (DeltaSeconds :type Float%20%28single-precision%29)))

(event EventInteract
  (params (Interactor :type BP%20Biologie%20First%20Person%20Character%20Object%20Reference))
  (bind _returnvalue (Game|GetPlayerController 0))
  (Utilities|Casting|CastToBP_BiologieFirstPersonCharacter Interactor)
  (if (== (Variables|Default|GetRecipeWidget) 0)
    (bind _returnvalue_2 (UserInterface|CreateWidget "/Game/MyStuff/Minigames/Biologie_Minigame/UI/WBP_RecipeBook.WBP_RecipeBook_C"))
    (bind _output_get (Variables|Default|SetRecipeWidget _returnvalue_2))
    (UserInterface|Viewport|AddtoViewport _output_get 0)
    (Input|SetInputModeUIOnly _returnvalue (Variables|Default|GetRecipeWidget) "DoNotLock" true)
    (Variables|/Script/Engine.PlayerController|SetbShowMouseCursor _returnvalue true)
    (Development|PrintString "interacted with book")
    (else
      (Variables|Default|SetRecipeWidget 0))))

(fn ConstructionScript)