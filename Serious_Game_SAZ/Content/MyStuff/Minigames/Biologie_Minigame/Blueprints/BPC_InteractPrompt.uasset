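; Actor component for the biology minigame that manages an interaction prompt shown through the owner's WidgetComponent.
; On BeginPlay it finds that component, casts its widget to WBP_InteractPrompt and applies the configured prompt text.
; Every tick it rotates the widget to face the player camera, billboard-style.
; ShowPrompt and HidePrompt toggle the widget's visibility after a validity check.
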(event EventTick
  (params (DeltaSeconds :type Float%20%28single-precision%29))
  (Transformation|SetWorldRotation (Variables|Default|GetWidgetComponentRef) (Math|Rotator|FindLookatRotation (Transformation|GetWorldLocation (Variables|Default|GetWidgetComponentRef)) (Camera|GetCameraLocation (Game|GetPlayerCameraManager 0))) false false))

(event EventBeginPlay
  (bind _output_get (Variables|Default|SetWidgetComponentRef (Actor|GetComponentbyClass (Components|GetOwner) "/Script/UMG.WidgetComponent")))
  (bind _aswbp_interact_prompt (Utilities|Casting|CastToWBP_InteractPrompt (UserInterface|GetUserWidgetObject _output_get)))
  (bind _output_get_2 (Variables|Default|SetPromptWidgetRef _aswbp_interact_prompt))
  (Default|SetPromptText _output_get_2 (Variables|Default|GetPromptText)))

(fn HidePrompt
  (bind _widgetcomponentref (Variables|Default|GetWidgetComponentRef))
  (Utilities|IsValid _widgetcomponentref
    (:Is%20Valid
      (Rendering|SetVisibility _widgetcomponentref false false))))

(fn ShowPrompt
  (bind _widgetcomponentref (Variables|Default|GetWidgetComponentRef))
  (Utilities|IsValid _widgetcomponentref
    (:Is%20Valid
      (Rendering|SetVisibility _widgetcomponentref true false))))