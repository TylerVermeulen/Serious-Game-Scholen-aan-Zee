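; BP_ItemDeposit is an interactable deposit point in the biology minigame where players hand in the item matching a displayed target.
; On BeginPlay it loads all rows of DT_TargetItems and picks a random target by shuffling, showing its icon through a dynamic material instance.
; Interacting compares the held item's ID to the target, plays a correct or incorrect sound, adds score on a match, then clears the item and picks a new target.
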(event EventBeginPlay
  ;[0.15 0.15 0.15 0.5] Sets data table into array
  (bind _outrownames (DataTable|GetDataTableRowNames "/Game/MyStuff/Minigames/Biologie_Minigame/Data/DT_TargetItems.DT_TargetItems"))
  (for _array_element _outrownames
    (bind _returnvalue (Utilities|GetDataTableRow "/Game/MyStuff/Minigames/Biologie_Minigame/Data/DT_TargetItems.DT_TargetItems" _array_element)
      (:then
        (Utilities|Array|Add (Variables|Default|GetTargets) _returnvalue))))
  (CallFunction|GenerateAnswer))

(event EventInteract
  (params (Interactor :type BP%20Biologie%20First%20Person%20Character%20Object%20Reference))
  ;[0.15 0.15 0.15 0.5] Checks if the item the player is holding matches the target item and gives points if correct
  (bind _output_get (Variables|Default|SetPlayer Interactor))
  (if (== (.itemid (Variables|/Game/MyStuff/Minigames/Biologie_Minigame/Blueprints/BP_BiologieFirstPersonCharacter.BP_BiologieFirstPersonCharacter_C|GetHeldItemData _output_get)) (.itemid (Variables|Default|GetTargetItem)))
    (Audio|PlaySound2D "/Game/MyStuff/Minigames/Geschiedenis_Minigame/Audio/SW_Correct.SW_Correct" 1.0 1.0 0.0 0 0)
    (bind _output_get_2 (Variables|/Game/MyStuff/Minigames/Biologie_Minigame/Blueprints/BP_BiologieFirstPersonCharacter.BP_BiologieFirstPersonCharacter_C|SetScore (Variables|Default|GetPlayer) (+ (Variables|/Game/MyStuff/Minigames/Biologie_Minigame/Blueprints/BP_BiologieFirstPersonCharacter.BP_BiologieFirstPersonCharacter_C|GetScore (Variables|Default|GetPlayer)) 1)))
    (Development|PrintString (Utilities|String|ToString(Integer) _output_get_2))
    (Default|ClearHeldItem (Variables|Default|GetPlayer))
    (CallFunction|GenerateAnswer)
    (else
      (Default|ClearHeldItem (Variables|Default|GetPlayer))
      (Audio|PlaySound2D "/Game/MyStuff/Minigames/Geschiedenis_Minigame/Audio/SW_Incorrect.SW_Incorrect" 1.0 1.0 0.0 0 0)
      (CallFunction|GenerateAnswer))))

(fn ConstructionScript
  (bind _returnvalue (Rendering|Material|CreateDynamicMaterialInstance (Variables|Default|GetTargetItemDisplay) 0 "/Game/MyStuff/Minigames/Biologie_Minigame/Materials/M_ItemDisplay.M_ItemDisplay" "None" :!class /Script/Engine.PrimitiveComponent))
  (Variables|Default|SetTargetItemMaterial _returnvalue))

(fn GenerateAnswer
  (bind _targets (Variables|Default|GetTargets))
  ;[0.15 0.15 0.15 0.5] Sets answer
  (Utilities|Array|Shuffle _targets)
  (bind _output_get (Variables|Default|SetTargetItem (Utilities|Array|Get(acopy) _targets)))
  (Rendering|Material|SetTextureParameterValue (Variables|Default|GetTargetItemMaterial) "ItemTexture" (.icon _output_get)))