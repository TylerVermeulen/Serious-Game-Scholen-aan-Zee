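; BP_ItemSource is an interactable item dispenser in the biology minigame that gives its configured item to the player.
; On Interact it passes ItemToGive to the interactor's PickupItemData if the hand is empty, otherwise it prints a "Hands full" message.
; The construction script creates a dynamic M_ItemDisplay material on the PreviewIcon and sets its texture to the item's icon.
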(event EventInteract
  (params (Interactor :type BP%20Biologie%20First%20Person%20Character%20Object%20Reference))
  ;[0.15 0.15 0.15 0.5] If hand is empty gives this items data to player character
  (if (== (Variables|/Game/MyStuff/Minigames/Biologie_Minigame/Blueprints/BP_BiologieFirstPersonCharacter.BP_BiologieFirstPersonCharacter_C|GetbHasItem Interactor) false)
    (Default|PickupItemData Interactor (Variables|Default|GetItemToGive))
    (else
      (Development|PrintString "Hands full"))))

(fn ConstructionScript
  (bind _returnvalue (Rendering|Material|CreateDynamicMaterialInstance (Variables|Default|GetPreviewIcon) 0 "/Game/MyStuff/Minigames/Biologie_Minigame/Materials/M_ItemDisplay.M_ItemDisplay" "None" :!class /Script/Engine.PrimitiveComponent))
  (bind _output_get (Variables|Default|SetPreviewIconMaterial _returnvalue))
  (Rendering|Material|SetMaterial (Variables|Default|GetPreviewIcon) 0 _output_get)
  (Rendering|Material|SetTextureParameterValue _returnvalue "ItemTexture" (.icon (Variables|Default|GetItemToGive))))