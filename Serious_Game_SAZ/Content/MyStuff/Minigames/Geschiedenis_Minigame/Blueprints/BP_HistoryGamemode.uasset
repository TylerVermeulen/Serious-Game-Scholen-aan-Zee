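; BP_HistoryGamemode is the game mode for the history (Geschiedenis) minigame and manages its start screen.
; On BeginPlay in GeschiedenisMap, it creates WBP_StartScreen if none exists, adds it to the viewport, and switches the player to UI-only input with a visible cursor.
; On EndPlay it prints the end reason and removes the start screen widget if it is still valid.
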(event EventBeginPlay
  (bind _returnvalue (Game|GetPlayerController 0))
  (bind _returnvalue_2 (Game|GetCurrentLevelName true))
  (if (Utilities|Enum|Equal(Enum) _returnvalue_2 (Variables|Default|GetGeschiedenisMap))
    (if (not (Utilities|IsValid (Variables|Default|GetStartScreenWidget)))
      (bind _returnvalue_3 (UserInterface|CreateWidget "/Game/MyStuff/Minigames/Geschiedenis_Minigame/UI/WBP_StartScreen.WBP_StartScreen_C"))
      (bind _output_get (Variables|Default|SetStartScreenWidget _returnvalue_3))
      (UserInterface|Viewport|AddtoViewport _output_get 0)
      (Input|SetInputModeUIOnly _returnvalue (Variables|Default|GetStartScreenWidget) "DoNotLock" false)
      (Variables|/Script/Engine.PlayerController|SetbShowMouseCursor _returnvalue true))))

(event EventEndPlay
  (params (EndPlayReason :type EEndPlayReason%20Enum :default "Destroyed"))
  (Development|PrintString (Utilities|String|EnumtoString EndPlayReason))
  (if (Utilities|IsValid (Variables|Default|GetStartScreenWidget))
    (Widget|RemovefromParent (Variables|Default|GetStartScreenWidget))))

(fn ConstructionScript)