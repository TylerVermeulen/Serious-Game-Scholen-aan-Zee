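; Quiz manager for the history (Geschiedenis) minigame, running timed multiple-choice questions from answer to final score.
; BeginPlay loads and shuffles DT_QuizQuestions; StartQuestion feeds the quiz screen widget and answer squares and starts a looping countdown timer.
; Submitted answers or timeouts show a result and advance the question.
; GameEnd records completion in GI_MinigameProgress, awards a game-wide point for a passing score and opens the exit door either way.
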(event EventBeginPlay
  ;[0.15 0.15 0.15 0.5] Grabs structs from the datatable. Then puts them into an array, shuffles them and then grabs the first one in the array to the current question
  (bind _returnvalue (Actor|GetActorOfClass "/Game/MyStuff/Minigames/Geschiedenis_Minigame/Blueprints/BP_QuizScreenActor.BP_QuizScreenActor_C"))
  (Variables|Default|SetQuizScreenRef _returnvalue)
  (bind _outrownames (DataTable|GetDataTableRowNames "/Game/MyStuff/Minigames/Geschiedenis_Minigame/Data/DT_QuizQuestions.DT_QuizQuestions"))
  (for _array_element _outrownames
    (bind _returnvalue_2 (Utilities|GetDataTableRow "/Game/MyStuff/Minigames/Geschiedenis_Minigame/Data/DT_QuizQuestions.DT_QuizQuestions" _array_element)
      (:then
        (Utilities|Array|Add (Variables|Default|GetQuestions) _returnvalue_2))))
  (Utilities|Array|Shuffle (Variables|Default|GetQuestions))
  (Variables|Default|SetCurrentQuestionIndex 0)
  (Utilities|FlowControl|Delay 0.3)
  (Default|SetQuestionTime (Variables|/Game/MyStuff/Minigames/Geschiedenis_Minigame/Blueprints/BP_QuizScreenActor.BP_QuizScreenActor_C|GetQuizWidgetRef (Variables|Default|GetQuizScreenRef)) (+ (Variables|Default|GetCurrentQuestionIndex) 1) (Utilities|Array|Length (Variables|Default|GetQuestions)))
  (Default|SetAnswersIntoArray (Variables|/Game/MyStuff/Minigames/Geschiedenis_Minigame/Blueprints/BP_QuizScreenActor.BP_QuizScreenActor_C|GetQuizWidgetRef (Variables|Default|GetQuizScreenRef))))

(fn ConstructionScript)

(fn StartQuestion
  ;[0.15 0.15 0.15 0.5] Gives all the data to neccesary scripts starts the timer
  (Variables|Default|SetCurrentQuestion (Utilities|Array|Get(acopy) (Variables|Default|GetQuestions) (Variables|Default|GetCurrentQuestionIndex)))
  (Default|ResetSquare (Variables|Default|GetAnswerSquares))
  (Variables|Default|SetBQuestionActive true)
  (Variables|Default|SetTimeRemaining (.timelimit (Variables|Default|GetCurrentQuestion)))
  (Default|SetQuestion (Variables|/Game/MyStuff/Minigames/Geschiedenis_Minigame/Blueprints/BP_QuizScreenActor.BP_QuizScreenActor_C|GetQuizWidgetRef (Variables|Default|GetQuizScreenRef)) (.questiontext (Variables|Default|GetCurrentQuestion)) (.answers (Variables|Default|GetCurrentQuestion)) (.correctindex (Variables|Default|GetCurrentQuestion)))
  (bind _returnvalue (Utilities|Time|SetTimerbyEvent (EventDispatchers|CreateEvent :!event TickQuestionTimer) 0.1 true))
  (Variables|Default|SetTimerHandle _returnvalue)
  (if (<= (Variables|Default|GetTimeRemaining) 0.0)
    _))

(fn SubmitAnsmer
  (params (Answerindex :type Integer))
  (bind _answerindex (LocalVariables|GetAnswerIndex))
  (bind _currentquestion (Variables|Default|GetCurrentQuestion))
  (bind _returnvalue (== _answerindex (.correctindex _currentquestion)))
  (Variables|Default|SetBQuestionActive false)
  (for _array_element (Variables|Default|GetAnswerSquares)
    (Default|DisableSquare _array_element))
  (if _returnvalue
    ;[0.15 0.15 0.15 0.5] If its correct it adds a point to the score and then waits 1.8 seconds till it starts the next question
    (Default|ShowResult (Variables|/Game/MyStuff/Minigames/Geschiedenis_Minigame/Blueprints/BP_QuizScreenActor.BP_QuizScreenActor_C|GetQuizWidgetRef (Variables|Default|GetQuizScreenRef)) _returnvalue Answerindex (.correctindex _currentquestion))
    (Variables|Default|SetScore (+ (Variables|Default|GetScore) 1))
    (Default|SetQuestionTime (Variables|/Game/MyStuff/Minigames/Geschiedenis_Minigame/Blueprints/BP_QuizScreenActor.BP_QuizScreenActor_C|GetQuizWidgetRef (Variables|Default|GetQuizScreenRef)) (+ (Variables|Default|GetCurrentQuestionIndex) 1) (Utilities|Array|Length (Variables|Default|GetQuestions)))
    (Utilities|Time|SetTimerbyEvent 0 1.8)
    (CallFunction|NextQuestion)
    (else
      ;[0.15 0.15 0.15 0.5] If its incorrect it only
      (Default|ShowResult (Variables|/Game/MyStuff/Minigames/Geschiedenis_Minigame/Blueprints/BP_QuizScreenActor.BP_QuizScreenActor_C|GetQuizWidgetRef (Variables|Default|GetQuizScreenRef)) _returnvalue Answerindex (.correctindex _currentquestion))
      (Default|SetQuestionTime (Variables|/Game/MyStuff/Minigames/Geschiedenis_Minigame/Blueprints/BP_QuizScreenActor.BP_QuizScreenActor_C|GetQuizWidgetRef (Variables|Default|GetQuizScreenRef)) (+ (Variables|Default|GetCurrentQuestionIndex) 1) (Utilities|Array|Length (Variables|Default|GetQuestions)))
      (Utilities|Time|SetTimerbyEvent 0 1.8)
      (CallFunction|NextQuestion))))

(fn NextQuestion
  (bind _output_get (Variables|Default|SetCurrentQuestionIndex (+ (Variables|Default|GetCurrentQuestionIndex) 1)))
  (if (< _output_get (Utilities|Array|Length (Variables|Default|GetQuestions)))
    (CallFunction|StartQuestion)
    (else
      (CallFunction|GameEnd))))

(fn TickQuestionTimer
  (bind _currentquestion (Variables|Default|GetCurrentQuestion))
  ;[0.15 0.15 0.15 0.5] Handles timer logic
  (Variables|Default|SetTimeRemaining (Math|Float|Clamp(Float) (- (Variables|Default|GetTimeRemaining) 0.1) 0.0 (.timelimit _currentquestion)))
  (Default|SetTimer (Variables|/Game/MyStuff/Minigames/Geschiedenis_Minigame/Blueprints/BP_QuizScreenActor.BP_QuizScreenActor_C|GetQuizWidgetRef (Variables|Default|GetQuizScreenRef)) (Math|Float|Clamp(Float) (- (Variables|Default|GetTimeRemaining) 0.1) 0.0 (.timelimit _currentquestion)) (.timelimit _currentquestion))
  (if (<= (Math|Float|Clamp(Float) (- (Variables|Default|GetTimeRemaining) 0.1) 0.0 (.timelimit _currentquestion)) 0.0)
    (Utilities|Time|ClearandInvalidateTimerbyHandle (Variables|Default|GetTimerHandle))
    (Default|ShowResult (Variables|/Game/MyStuff/Minigames/Geschiedenis_Minigame/Blueprints/BP_QuizScreenActor.BP_QuizScreenActor_C|GetQuizWidgetRef (Variables|Default|GetQuizScreenRef)) false)
    (Utilities|Time|SetTimerbyEvent 0 1.8)
    (CallFunction|NextQuestion)))

(fn StartQuiz
  (CallFunction|StartQuestion))

(fn GameEnd
  (bind _quizscreenref (Variables|Default|GetQuizScreenRef))
  (bind _score (Variables|Default|GetScore))
  (bind _quizwidgetref (Variables|/Game/MyStuff/Minigames/Geschiedenis_Minigame/Blueprints/BP_QuizScreenActor.BP_QuizScreenActor_C|GetQuizWidgetRef _quizscreenref))
  ;[0.15 0.15 0.15 0.5] SetsText to score and check if you won
  (Rendering|Components|TextRender|SetText (Variables|/Game/MyStuff/Minigames/Geschiedenis_Minigame/UI/WBP_QuizScreen.WBP_QuizScreen_C|GetPuntenTextBlock (Variables|/Game/MyStuff/Minigames/Geschiedenis_Minigame/Blueprints/BP_QuizScreenActor.BP_QuizScreenActor_C|GetQuizWidgetRef (Variables|Default|GetQuizScreenRef))) (Utilities|Text|ToText(Integer) _score))
  (bind _asgi_minigame_progress (Utilities|Casting|CastToGI_MinigameProgress (Game|GetGameInstance)))
  (Variables|/Game/MyStuff/CentralHub/Blueprints/GI_MinigameProgress.GI_MinigameProgress_C|SetbHistoryDone _asgi_minigame_progress true)
  (if (>= _score 6)
    ;[0.15 0.15 0.15 0.5] Opens Exitdoor and if you won the quiz give big point for whole game
    (Variables|Default|SetBWonGame true)
    (bind _asgi_minigame_progress_2 (Utilities|Casting|CastToGI_MinigameProgress (Game|GetGameInstance)))
    (Utilities|Array|AddUnique (Variables|/Game/MyStuff/CentralHub/Blueprints/GI_MinigameProgress.GI_MinigameProgress_C|GetCompletedGames _asgi_minigame_progress_2) "GeschiedenisGame")
    (Variables|/Game/MyStuff/CentralHub/Blueprints/GI_MinigameProgress.GI_MinigameProgress_C|SetTotalPoints _asgi_minigame_progress_2 (+ (Variables|/Game/MyStuff/CentralHub/Blueprints/GI_MinigameProgress.GI_MinigameProgress_C|GetTotalPoints _asgi_minigame_progress_2) 1))
    (Variables|Default|SetBGameEnd true)
    (bind _returnvalue (Actor|GetActorOfClass "/Game/MyStuff/Minigames/Geschiedenis_Minigame/Blueprints/BP_ExitDoorHistory.BP_ExitDoorHistory_C"))
    (Default|AllowExit _returnvalue)
    (Widget|SetVisibility (Variables|/Game/MyStuff/Minigames/Geschiedenis_Minigame/UI/WBP_QuizScreen.WBP_QuizScreen_C|GetWinnerTextBlock _quizwidgetref) "Visible")
    (Widget|SetVisibility (Variables|/Game/MyStuff/Minigames/Geschiedenis_Minigame/UI/WBP_QuizScreen.WBP_QuizScreen_C|GetGameOverScreen _quizwidgetref) "Visible")
    (else
      ;[0.15 0.15 0.15 0.5] Opens the exitdoor
      (Variables|Default|SetBWonGame false)
      (Variables|Default|SetBGameEnd true)
      (bind _returnvalue_2 (Actor|GetActorOfClass "/Game/MyStuff/Minigames/Geschiedenis_Minigame/Blueprints/BP_ExitDoorHistory.BP_ExitDoorHistory_C"))
      (Default|AllowExit _returnvalue_2)
      (Widget|SetVisibility (Variables|/Game/MyStuff/Minigames/Geschiedenis_Minigame/UI/WBP_QuizScreen.WBP_QuizScreen_C|GetGameOverScreen (Variables|/Game/MyStuff/Minigames/Geschiedenis_Minigame/Blueprints/BP_QuizScreenActor.BP_QuizScreenActor_C|GetQuizWidgetRef (Variables|Default|GetQuizScreenRef))) "Visible")
      (bind _asgi_minigame_progress_3 (Utilities|Casting|CastToGI_MinigameProgress (Game|GetGameInstance)))
      (Utilities|Array|AddUnique (Variables|/Game/MyStuff/CentralHub/Blueprints/GI_MinigameProgress.GI_MinigameProgress_C|GetCompletedGames _asgi_minigame_progress_3) "GeschiedenisGame"))))