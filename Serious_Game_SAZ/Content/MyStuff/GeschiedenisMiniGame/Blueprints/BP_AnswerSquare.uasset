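; BP_AnswerSquare is a trigger square for the history quiz minigame that the first-person character steps on to choose an answer.
; It finds BP_QuizManager on BeginPlay and, when overlapped while unlocked during an active question, submits its AnswerIndex to the manager after a short delay.
; DisableSquare and ResetSquare events toggle the lock and box collision to block or re-allow answers.
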(event OnComponentBeginOverlap(Box)
  (params (OverlappedComponent :type Primitive%20Component%20Object%20Reference) (OtherActor :type Actor%20Object%20Reference) (OtherComp :type Primitive%20Component%20Object%20Reference) (OtherBodyIndex :type Integer) (bFromSweep :type Boolean) (SweepResult :type Hit%20Result%20Structure%20%28by%20ref%29))
  (Utilities|Casting|CastToBP_FirstPersonCharacter OtherActor)
  (if (== (Variables|Default|GetbLocked) false)
    (if (== (Variables|/Game/MyStuff/GeschiedenisMiniGame/Blueprints/BP_QuizManager.BP_QuizManager_C|GetBQuestionActive (Variables|Default|GetQuizmanagerRef)) true)
      (Utilities|FlowControl|Delay 0.3)
      (Default|SubmitAnsmer (Variables|Default|GetQuizmanagerRef) (Variables|Default|GetAnswerIndex)))))

(event Custom|DisableSquare
  ;[0.15 0.15 0.15 0.5] Disables Collision when player touches a square
  (Variables|Default|SetbLocked true)
  (Collision|SetCollisionEnabled (Variables|Default|GetBox) "NoCollision"))

(event Custom|ResetSquare
  ;[0.15 0.15 0.15 0.5] Reenables collision after question has been proccessed
  (Variables|Default|SetbLocked false)
  (Collision|SetCollisionEnabled (Variables|Default|GetBox) "QueryOnly"))

(event EventBeginPlay
  (bind _returnvalue (Actor|GetActorOfClass "/Game/MyStuff/GeschiedenisMiniGame/Blueprints/BP_QuizManager.BP_QuizManager_C"))
  (Variables|Default|SetQuizmanagerRef _returnvalue))

(event Collision|EventActorBeginOverlap
  (params (OtherActor :type Actor%20Object%20Reference)))

(fn ConstructionScript)