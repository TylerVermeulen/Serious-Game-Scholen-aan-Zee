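; Quiz manager for a history minigame that runs timed multiple-choice questions on a quiz screen actor's widget.
; It loads and shuffles questions from DT_QuizQuestions, then resets the answer squares and starts a looping countdown timer for each question.
; Submitted answers disable the squares, show the result, update the score and advance, printing the final score after the last question.
; Timer expiry only stops the countdown, without submitting or advancing.
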(event EventBeginPlay
  (bind _returnvalue (Actor|GetActorOfClass "/Game/MyStuff/GeschiedenisMiniGame/Blueprints/BP_QuizScreenActor.BP_QuizScreenActor_C"))
  (Variables|Default|SetQuizScreenRef _returnvalue)
  (bind _outrownames (DataTable|GetDataTableRowNames "/Game/MyStuff/GeschiedenisMiniGame/Data/DT_QuizQuestions.DT_QuizQuestions"))
  (for _array_element _outrownames
    (bind _returnvalue_2 (Utilities|GetDataTableRow "/Game/MyStuff/GeschiedenisMiniGame/Data/DT_QuizQuestions.DT_QuizQuestions" _array_element)
      (:then
        (Utilities|Array|Add (Variables|Default|GetQuestions) _returnvalue_2))))
  (Utilities|Array|Shuffle (Variables|Default|GetQuestions))
  (Variables|Default|SetCurrentQuestionIndex 0)
  (Default|SetScore (Variables|/Game/MyStuff/GeschiedenisMiniGame/Blueprints/BP_QuizScreenActor.BP_QuizScreenActor_C|GetQuizWidgetRef (Variables|Default|GetQuizScreenRef)) (Variables|Default|GetScore) (Utilities|Array|Length (Variables|Default|GetQuestions)))
  (Default|SetAnswersIntoArray (Variables|/Game/MyStuff/GeschiedenisMiniGame/Blueprints/BP_QuizScreenActor.BP_QuizScreenActor_C|GetQuizWidgetRef (Variables|Default|GetQuizScreenRef)))
  (CallFunction|StartQuestion))

(fn ConstructionScript)

(fn StartQuestion
  (Variables|Default|SetCurrentQuestion (Utilities|Array|Get(acopy) (Variables|Default|GetQuestions) (Variables|Default|GetCurrentQuestionIndex)))
  (Default|ResetSquare (Variables|Default|GetAnswerSquares))
  (Variables|Default|SetBQuestionActive true)
  (Variables|Default|SetTimeRemaining (.timelimit (Variables|Default|GetCurrentQuestion)))
  (Default|SetQuestion (Variables|/Game/MyStuff/GeschiedenisMiniGame/Blueprints/BP_QuizScreenActor.BP_QuizScreenActor_C|GetQuizWidgetRef (Variables|Default|GetQuizScreenRef)) (.questiontext (Variables|Default|GetCurrentQuestion)) (.answers (Variables|Default|GetCurrentQuestion)) (.correctindex (Variables|Default|GetCurrentQuestion)))
  (bind _returnvalue (Utilities|Time|SetTimerbyFunctionName 0 "TickQuestionTimer" 0.1 true))
  (Variables|Default|SetTimerHandle _returnvalue)
  (bind _output_get (Variables|Default|SetTimeRemaining 0.0))
  (if (<= _output_get 0.0)
    _))

(fn SubmitAnsmer
  (params (Answerindex :type Integer))
  (bind _answerindex (LocalVariables|GetAnswerIndex))
  (bind _currentquestion (Variables|Default|GetCurrentQuestion))
  (bind _returnvalue (== _answerindex (.correctindex _currentquestion)))
  (Variables|Default|SetBQuestionActive false)
  (for _array_element (Variables|Default|GetAnswerSquares)
    (Default|DisableSquare _array_element))
  (if _returnvalue
    (Default|ShowResult (Variables|/Game/MyStuff/GeschiedenisMiniGame/Blueprints/BP_QuizScreenActor.BP_QuizScreenActor_C|GetQuizWidgetRef (Variables|Default|GetQuizScreenRef)) _returnvalue Answerindex (.correctindex _currentquestion))
    (bind _output_get (Variables|Default|SetScore (+ (Variables|Default|GetScore) 1)))
    (Default|SetScore (Variables|/Game/MyStuff/GeschiedenisMiniGame/Blueprints/BP_QuizScreenActor.BP_QuizScreenActor_C|GetQuizWidgetRef (Variables|Default|GetQuizScreenRef)) _output_get (Utilities|Array|Length (Variables|Default|GetQuestions)))
    (Utilities|Time|SetTimerbyEvent 0 1.8)
    (CallFunction|NextQuestion)
    (else
      (Default|ShowResult (Variables|/Game/MyStuff/GeschiedenisMiniGame/Blueprints/BP_QuizScreenActor.BP_QuizScreenActor_C|GetQuizWidgetRef (Variables|Default|GetQuizScreenRef)) _returnvalue Answerindex (.correctindex _currentquestion))
      (Utilities|Time|SetTimerbyEvent 0 1.8)
      (CallFunction|NextQuestion))))

(fn NextQuestion
  (bind _output_get (Variables|Default|SetCurrentQuestionIndex (+ (Variables|Default|GetCurrentQuestionIndex) 1)))
  (if (< _output_get (Utilities|Array|Length (Variables|Default|GetQuestions)))
    (CallFunction|StartQuestion)
    (else
      (Development|PrintString "Games over 
Final score is ")
      (Development|PrintString (Utilities|String|ToString(Integer) (Variables|Default|GetScore)))
      (Development|PrintString "out of 6"))))

(fn TickQuestionTimer
  (bind _currentquestion (Variables|Default|GetCurrentQuestion))
  (Variables|Default|SetTimeRemaining (Math|Float|Clamp(Float) (- (Variables|Default|GetTimeRemaining) 0.1) 0.0 (.timelimit _currentquestion)))
  (Default|SetTimer (Variables|/Game/MyStuff/GeschiedenisMiniGame/Blueprints/BP_QuizScreenActor.BP_QuizScreenActor_C|GetQuizWidgetRef (Variables|Default|GetQuizScreenRef)) (Math|Float|Clamp(Float) (- (Variables|Default|GetTimeRemaining) 0.1) 0.0 (.timelimit _currentquestion)) (.timelimit _currentquestion))
  (if (<= (Math|Float|Clamp(Float) (- (Variables|Default|GetTimeRemaining) 0.1) 0.0 (.timelimit _currentquestion)) 0.0)
    (Utilities|Time|ClearandInvalidateTimerbyHandle (Variables|Default|GetTimerHandle))))